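; BP_FishingPond is a fishing pond actor that repositions its Chair relative to the pond's static mesh when play begins.
; On BeginPlay it multiplies the chair's world offset from the mesh by RadiusXYScale and teleport-free, sweep-free moves the chair to that point.
; The construction script is empty, so the adjustment happens only at runtime, and no fishing logic is present in these graphs.
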(event `self.ReceiveBeginPlay`
  (bind _returnvalue (`SceneComponent.K2_GetComponentLocation` (`self.StaticMeshComponent`)))
  (`SceneComponent.K2_SetWorldLocation` (`self.Chair`) (+ _returnvalue (* (- (`SceneComponent.K2_GetComponentLocation` (`self.Chair`)) _returnvalue) (`self.RadiusXYScale`))) false false))

(fn `UserConstructionScript`)